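; Behavior Tree task that makes an enemy inspect a zone by turning its pawn to look to one side, then the other.
; Each tick it eases the controlled pawn's yaw with RInterpTo toward 90, then -90 degrees, as absolute world angles rather than offsets from its facing.
; Two flags, reset on execute, advance when rotation is within tolerance, and the task finishes successfully once both are set.
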(event `self.ReceiveExecute`
  (params (OwnerActor :type "Actor Object Reference"))
  (set `self.bLeftSearch` false)
  (set `self.bRightSearch` false))

(event `self.ReceiveTick`
  (params (OwnerActor :type "Actor Object Reference") (DeltaSeconds :type "Float (single-precision)"))
  (if (`self.bLeftSearch`)
    (if (`self.bRightSearch`)
      (`self.FinishExecute` true)
      (else
        (`self.LookAtOneAngle` -90.0 OwnerActor DeltaSeconds)))
    (else
      (`self.LookAtOneAngle` 90.0 OwnerActor DeltaSeconds))))

(fn `LookAtOneAngle`
  (params (Angle :type "Float (double-precision)") (ActorOwner :type "Actor Object Reference") (DeltaSeconds :type "Float (double-precision)"))
  (bind _asenemy_aicontroller (cast `EnemyAIController` ActorOwner))
  (bind _returnvalue (`Controller.K2_GetPawn` _asenemy_aicontroller))
  (bind _returnvalue_2 (`Actor.K2_GetActorRotation` _returnvalue))
  (bind _returnvalue_3 (`KismetMathLibrary.MakeRotator` (.roll _returnvalue_2) (.pitch _returnvalue_2) Angle))
  (bind _returnvalue_4 (`KismetMathLibrary.RInterpTo` _returnvalue_2 _returnvalue_3 DeltaSeconds 2.0))
  (`Actor.K2_SetActorRotation` _returnvalue _returnvalue_4 false)
  (if (not (!= _returnvalue_4 _returnvalue_3 :`ErrorTolerance` 20.0))
    (if (`self.bLeftSearch`)
      (set `self.bRightSearch` true)
      (else
        (set `self.bLeftSearch` true)))))