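; Behavior Tree task for unit AI that publishes the front entry of the unit's action queue to the Blackboard.
; On execute it casts the owner to UnitAIController and copies the first ActionsManager queue entry's action and destination into the CurrentAction and TargetLocation keys.
; It then finishes successfully, without removing the entry or checking for an empty queue.
; A failed cast never calls FinishExecute.
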(event `self.ReceiveExecute`
  (params (OwnerActor :type "Actor Object Reference"))
  (bind _asunit_aicontroller (cast `UnitAIController` OwnerActor))
  (bind _blackboardcomponent (`UnitAIController.BlackboardComponent` _asunit_aicontroller))
  (bind (_action _instigator _target _destiny) (break `ActionInformation` (`|GetArrayItem` (`ActionsComponent.ActionQueue` (`UnitAIController.ActionsManager` _asunit_aicontroller)))))
  (`BlackboardComponent.SetValueAsEnum` _blackboardcomponent "CurrentAction" _action)
  (`BlackboardComponent.SetValueAsVector` _blackboardcomponent "TargetLocation" _destiny)
  (`self.FinishExecute` true))