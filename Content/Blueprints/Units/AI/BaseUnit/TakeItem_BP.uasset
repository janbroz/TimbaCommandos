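; Behavior tree task that has an AI-controlled unit walk to an item and pick it up.
; On execute, it takes the target of the first entry in the controller's ActionsManager queue and starts a move toward it.
; Tick polls pawn distance, adds the item to the BaseUnit's InventoryManager when close and finishes successfully, otherwise printing the distance.
; It has no failure finish.
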(event `self.ReceiveTick`
  (params (OwnerActor :type "Actor Object Reference") (DeltaSeconds :type "Float (single-precision)"))
  (bind _itemtarget (`self.ItemTarget`))
  (bind _asaicontroller (cast `AIController` OwnerActor))
  (bind _returnvalue (`Controller.K2_GetPawn` _asaicontroller))
  (bind _returnvalue_2 (`Actor.GetDistanceTo` _returnvalue (`self.ItemTarget`)))
  (if (< _returnvalue_2 180.0)
    (bind _asbase_unit (cast `BaseUnit` _returnvalue))
    (if (`KismetSystemLibrary.IsValid` _itemtarget)
      (bind _asitem (cast `Item` _itemtarget))
      (`InventoryManager.AddItem` (`BaseUnit.InventoryManager` _asbase_unit) _asitem)
      (`self.FinishExecute` true))
    (else
      (`KismetSystemLibrary.PrintString` (`KismetStringLibrary.Conv_DoubleToString` _returnvalue_2)))))

(event `self.ReceiveExecute`
  (params (OwnerActor :type "Actor Object Reference"))
  (`KismetSystemLibrary.PrintString` "They called take items")
  (bind _asunit_aicontroller (cast `UnitAIController` OwnerActor))
  (bind (_action _instigator _target) (break `ActionInformation` (`|GetArrayItem` (`ActionsComponent.ActionQueue` (`UnitAIController.ActionsManager` _asunit_aicontroller)))))
  (`AIController.MoveToActor` _asunit_aicontroller _target 150.0 true true true null true)
  (set `self.ItemTarget` _target))