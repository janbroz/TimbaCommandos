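; Carriage is a test actor that travels along a referenced SplineActor's spline and calls OpenDoor on another object when its run ends.
; Each Tick it aligns to the spline direction nearest its Cube, then moves along the Cube's forward vector at Speed.
; Progress accumulates only the world X component of movement and is compared, with an offset, to spline length.
; Disconnected timeline logic for raising and reversing a door never runs.
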(event `self.ReceiveTick`
  (params (DeltaSeconds :type "Float (single-precision)"))
  (bind _cube (`self.Cube`))
  (bind _returnvalue (* (* (`SceneComponent.GetForwardVector` _cube) DeltaSeconds) (`self.Speed`)))
  (bind _asspline_actor (cast `/Game/Blueprints/Testing/SplineActor` (`self.SplineActor`)))
  (bind _spline (`/Game/Blueprints/Testing/SplineActor.Spline` _asspline_actor))
  (if (< (`KismetMathLibrary.Abs` (+ (`self.Distance`) -400.0)) (`SplineComponent.GetSplineLength` _spline))
    (`self.K2_SetActorRotation` (`KismetMathLibrary.Conv_VectorToRotator` (`SplineComponent.FindDirectionClosestToWorldLocation` _spline (`SceneComponent.K2_GetComponentLocation` _cube) "World")))
    (`self.K2_SetActorLocation` (+ (`self.K2_GetActorLocation`) _returnvalue))
    (set `self.Distance` (+ (`self.Distance`) (.x _returnvalue)))
    (else
      (`/Game/Blueprints/Testing/Door.OpenDoor` (`self.NewVar_0`)))))

(fn `UserConstructionScript`)