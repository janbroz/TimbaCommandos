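; Test door Blueprint that slides its mesh upward when OpenDoor is called.
; The construction script caches the mesh's world location and a raised destination, and a timeline lerps between them.
; OpenDoor and CloseDoor wrap custom events, but the closing event is empty.
; An InterpToMovement stop event prints a debug string, then calls CloseDoor after a delay, with no resulting movement.
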(event `self.InterpToMovement.OnInterpToStop`
  (params (ImpactResult :type "HitResult Structure (by ref)") (Time :type "Float (single-precision)"))
  (`KismetSystemLibrary.PrintString` "Nigga, im done")
  (`KismetSystemLibrary.Delay` 2.0)
  (`self.CloseDoor`))

(event `OpenTheDoor`
  (bind (_direction _alpha) (`Timeline|DoorOpening`)
    (:`Update`
      (`SceneComponent.K2_SetWorldLocation` (`self.DoorMesh`) (`KismetMathLibrary.VLerp` (`self.InitialLocation`) (`self.Destination`) _alpha) false false))))

(event `CloseTheDoor`)

(fn `CloseDoor`
  (`self.CloseTheDoor`))

(fn `OpenDoor`
  (`self.OpenTheDoor`))

(fn `UserConstructionScript`
  (bind _returnvalue (`SceneComponent.K2_GetComponentLocation` (`self.DoorMesh`)))
  (set `self.InitialLocation` _returnvalue)
  (set `self.Destination` (+ _returnvalue (0.0 0.0 600.0))))