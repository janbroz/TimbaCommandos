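; Apple is an item Blueprint whose use succeeds only when its quest target NPC is nearby.
; UseItem overrides the parent without calling it, searching all NPCUnit actors for QuestTarget and comparing a distance against UsableDistance.
; A match within range prints a debug message and returns true; otherwise it returns false, with no other effect on the item or quest.
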(fn `UseItem`
  (params (Target :type "Actor Object Reference"))
  (returns (ReturnValue :type Boolean))
  (bind _outactors (`GameplayStatics.GetAllActorsOfClass` "/Script/TimbaCommandos.NPCUnit"))
  (for _array_element _outactors
    (if (== _array_element (`self.QuestTarget`))
      (if (< (`self.GetDistanceTo` null) (`self.UsableDistance`))
        (`KismetSystemLibrary.PrintString` "The NPC is in the scene and close to us")
        (return true))))
  (return false))

(fn `UserConstructionScript`)